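; BP_Note_Maker is a note actor that lets the player show a note card while overlapping it.
; Begin overlap enables input on the actor and copies its NodeCard value into the top-down character's NoteCardIndex.
; R uses a FlipFlop to create or remove the NoteCardDisplay widget.
; End overlap disables input and removes the widget without resetting the FlipFlop, and neither overlap event checks which actor triggered it.
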(event Collision|EventActorBeginOverlap
  (params (OtherActor :type Actor%20Object%20Reference))
  (Input|EnableInput (Game|GetPlayerController 0))
  (bind _asbp_top_down_character (Utilities|Casting|CastToBP_TopDownCharacter (Game|GetPlayerCharacter 0)))
  (Variables|/Game/TopDown/Blueprints/BP_TopDownCharacter.BP_TopDownCharacter_C|SetNoteCardIndex _asbp_top_down_character (Variables|Default|GetNodeCard)))

(event Collision|EventActorEndOverlap
  (params (OtherActor :type Actor%20Object%20Reference))
  (Input|DisableInput 0)
  (Widget|RemovefromParent (stale Input|KeyboardEvents|R _returnvalue)))

(event Input|KeyboardEvents|R
  (params (Key :type Key%20Structure :default "None"))
  (:Pressed
    (Utilities|FlowControl|FlipFlop
      (:A
        (bind _returnvalue (UserInterface|CreateWidget "/Game/NoteCardDisplay.NoteCardDisplay_C"))
        (UserInterface|Viewport|AddtoViewport _returnvalue 0))
      (:B
        (Widget|RemovefromParent _returnvalue)))))

(fn ConstructionScript)